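; Player controller Blueprint for UntilYouBreak that manages the HUD and the end-of-game result screen.
; On BeginPlay it creates the HUD, caches its score widget and seeds the remaining enemy count from BP_UBGameMode.
; Score and retry-count events update that widget.
; Game-over and game-clear events share one path that shows the result widget with failure or success and clears all Enhanced Input mappings.
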(event Custom|OnGameOver
  (Variables|Default|SetIs%20Success false)
  (bind _returnvalue (UserInterface|CreateWidget "/Game/UntilYouBreak/UI/WBP_GameResult.WBP_GameResult_C" (Game|GetPlayerController 0)))
  (UserInterface|Viewport|AddtoViewport _returnvalue 0)
  (Default|SetResult _returnvalue (Variables|Default|GetIs%20Success))
  (Class|EnhancedInputSubsystemInterface|ClearAllMappings (PlayerController|LocalPlayerSubsystems|GetEnhancedInputLocalPlayerSubsystem)))

(event Custom|OnGameClear
  (Variables|Default|SetIs%20Success true)
  (bind _returnvalue (UserInterface|CreateWidget "/Game/UntilYouBreak/UI/WBP_GameResult.WBP_GameResult_C" (Game|GetPlayerController 0)))
  (UserInterface|Viewport|AddtoViewport _returnvalue 0)
  (Default|SetResult _returnvalue (Variables|Default|GetIs%20Success))
  (Class|EnhancedInputSubsystemInterface|ClearAllMappings (PlayerController|LocalPlayerSubsystems|GetEnhancedInputLocalPlayerSubsystem)))

(event Custom|OnNewScore
  (Default|SetRemainingEnemyCount (Variables|Default|GetScoreWidget) (stale EventOnScoreChanged NewScore)))

(event EventBeginPlay
  (bind _returnvalue (UserInterface|CreateWidget "/Game/UntilYouBreak/UI/WBP_UBHUD.WBP_UBHUD_C"))
  (UserInterface|Viewport|AddtoViewport _returnvalue 0)
  (Variables|Default|SetScoreWidget (Variables|/Game/UntilYouBreak/UI/WBP_UBHUD.WBP_UBHUD_C|GetWBP_PlayerScore _returnvalue))
  (bind _asbp_ubgame_mode (Utilities|Casting|CastToBP_UBGameMode (Game|GetGameMode)))
  (Default|SetRemainingEnemyCount (Variables|Default|GetScoreWidget) (Variables|/Script/UntilYouBreak.UBGameMode|GetRemainingEnemyCount _asbp_ubgame_mode)))

(event EventTick
  (params (DeltaSeconds :type Float%20%28single-precision%29)))

(event EventOnGameOver
  (Variables|Default|SetIs%20Success false)
  (bind _returnvalue (UserInterface|CreateWidget "/Game/UntilYouBreak/UI/WBP_GameResult.WBP_GameResult_C" (Game|GetPlayerController 0)))
  (UserInterface|Viewport|AddtoViewport _returnvalue 0)
  (Default|SetResult _returnvalue (Variables|Default|GetIs%20Success))
  (Class|EnhancedInputSubsystemInterface|ClearAllMappings (PlayerController|LocalPlayerSubsystems|GetEnhancedInputLocalPlayerSubsystem)))

(event EventOnGameClear
  (Variables|Default|SetIs%20Success true)
  (bind _returnvalue (UserInterface|CreateWidget "/Game/UntilYouBreak/UI/WBP_GameResult.WBP_GameResult_C" (Game|GetPlayerController 0)))
  (UserInterface|Viewport|AddtoViewport _returnvalue 0)
  (Default|SetResult _returnvalue (Variables|Default|GetIs%20Success))
  (Class|EnhancedInputSubsystemInterface|ClearAllMappings (PlayerController|LocalPlayerSubsystems|GetEnhancedInputLocalPlayerSubsystem)))

(event EventOnGameRetryCount
  (params (NewRetryCount :type Integer))
  (Default|SetRetryCount (Variables|Default|GetScoreWidget) NewRetryCount))

(event EventOnScoreChanged
  (params (NewScore :type Integer))
  (Default|SetRemainingEnemyCount (Variables|Default|GetScoreWidget) NewScore))

(fn ConstructionScript)